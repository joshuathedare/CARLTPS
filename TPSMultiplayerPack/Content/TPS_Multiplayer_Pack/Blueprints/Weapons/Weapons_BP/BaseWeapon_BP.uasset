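; Base multiplayer weapon that fires rifle or shotgun projectiles from the muzzle toward the player's aim point.
; FireRifle and FireShotgun trace from the camera along control rotation, with shotgun shots adding random cone spread.
; Clients send the computed transform to server events, which spawn the projectile with a jittered location and pass it damage, crit and impact values.
; StopFireWeapon is empty, and Server_StartFire only prints debug text.
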(event Custom|FireRifle
  (bind _projectilespawninfo (CallFunction|CalcaulateShootingInfoServer))
  (Variables|Default|SetTransform _projectilespawninfo)
  (Networking|SwitchHasAuthority
    (:Authority
      (bind _returnvalue (CallFunction|RandomizeVector (.location (Variables|Default|GetTransform))))
      (bind _returnvalue_2 (Game|SpawnActorfromClass (Variables|Default|GetProjectileClass) (Math|Transform|MakeTransform _returnvalue (.rotation (Variables|Default|GetTransform)) (.scale (Variables|Default|GetTransform))) "AlwaysSpawn" 0 (Game|GetInstigator)))
      (Default|SetDamageInfo _returnvalue_2 (Variables|Default|GetDamageMin) (Variables|Default|GetDamageMax) (Variables|Default|GetCritChance) (Variables|Default|GetImpactForce)))
    (:Remote
      (CallFunction|ServerFireRifle _projectilespawninfo))))

(event Custom|StopFireWeapon)

(event Custom|ServerFireRifle
  (params (Transform :type Transform))
  (Variables|Default|SetTransform Transform)
  (Networking|SwitchHasAuthority
    (:Authority
      (bind _returnvalue (CallFunction|RandomizeVector (.location (Variables|Default|GetTransform))))
      (bind _returnvalue_2 (Game|SpawnActorfromClass (Variables|Default|GetProjectileClass) (Math|Transform|MakeTransform _returnvalue (.rotation (Variables|Default|GetTransform)) (.scale (Variables|Default|GetTransform))) "AlwaysSpawn" 0 (Game|GetInstigator)))
      (Default|SetDamageInfo _returnvalue_2 (Variables|Default|GetDamageMin) (Variables|Default|GetDamageMax) (Variables|Default|GetCritChance) (Variables|Default|GetImpactForce)))
    (:Remote
      (CallFunction|ServerFireRifle (stale Custom|FireRifle _projectilespawninfo)))))

(event Custom|FireShotgun
  (bind _projectilespawninfo (CallFunction|CalcaulateShootingInfoShotgun))
  (Variables|Default|SetTransform _projectilespawninfo)
  (Networking|SwitchHasAuthority
    (:Authority
      (bind _returnvalue (CallFunction|RandomizeVector (.location (Variables|Default|GetTransform))))
      (bind _returnvalue_2 (Game|SpawnActorfromClass (Variables|Default|GetProjectileClass) (Math|Transform|MakeTransform _returnvalue (.rotation (Variables|Default|GetTransform)) (.scale (Variables|Default|GetTransform))) "AlwaysSpawn" 0 (Game|GetInstigator)))
      (Default|SetDamageInfo _returnvalue_2 (Variables|Default|GetDamageMin) (Variables|Default|GetDamageMax) (Variables|Default|GetCritChance) (Variables|Default|GetImpactForce)))
    (:Remote
      (CallFunction|ServerFireShotgun _projectilespawninfo))))

(event Custom|ServerFireShotgun
  (params (Transform :type Transform))
  (Variables|Default|SetTransform Transform)
  (Networking|SwitchHasAuthority
    (:Authority
      (bind _returnvalue (CallFunction|RandomizeVector (.location (Variables|Default|GetTransform))))
      (bind _returnvalue_2 (Game|SpawnActorfromClass (Variables|Default|GetProjectileClass) (Math|Transform|MakeTransform _returnvalue (.rotation (Variables|Default|GetTransform)) (.scale (Variables|Default|GetTransform))) "AlwaysSpawn" 0 (Game|GetInstigator)))
      (Default|SetDamageInfo _returnvalue_2 (Variables|Default|GetDamageMin) (Variables|Default|GetDamageMax) (Variables|Default|GetCritChance) (Variables|Default|GetImpactForce)))
    (:Remote
      (CallFunction|ServerFireShotgun (stale Custom|FireShotgun _projectilespawninfo)))))

(fn ConstructionScript)

(fn CalcaulateShootingInfo
  (bind _playercamera (Variables|Default|GetPlayerCamera))
  (bind _weaponmesh (Variables|Default|GetWeaponMesh))
  (bind _returnvalue (Transformation|GetWorldLocation _playercamera))
  (bind _returnvalue_2 (Math|Vector|GetForwardVector _playercamera))
  (bind _returnvalue_3 (Transformation|GetSocketLocation _weaponmesh "Muzzle"))
  (bind _returnvalue_4 (* _returnvalue_2 1e+04))
  (bind _returnvalue_5 (+ _returnvalue _returnvalue_4))
  (bind (_outhit _returnvalue_6) (Collision|LineTraceByChannel _returnvalue _returnvalue_5 "TraceTypeQuery3" false 0 "None"))
  (if _returnvalue_6
    (return (Math|Transform|MakeTransform _returnvalue_3 (Math|Rotator|FindLookatRotation _returnvalue_3 (.ImpactPoint (Collision|BreakHitResult _outhit)))))
    (else
      (return (Math|Transform|MakeTransform _returnvalue_3 (Math|Rotator|FindLookatRotation _returnvalue_3 _returnvalue_5))))))

(fn SetCameraandOwner
  (params (OwningCharacter :type PB%20Player%20Character%20Object%20Reference) (InputCamera :type Camera%20Component%20Object%20Reference))
  (bind _output_get (Variables|Default|SetOwning%20Character OwningCharacter))
  (Variables|Default|SetPlayerCamera InputCamera)
  (Actor|SetOwner _output_get))

(fn CalcaulateShootingInfoShotgun
  (bind _playercamera (Variables|Default|GetPlayerCamera))
  (bind _owning_character (Variables|Default|GetOwning%20Character))
  (bind _weaponmesh (Variables|Default|GetWeaponMesh))
  (bind _weaponmesh_2 (Variables|Default|GetWeaponMesh))
  (bind _weaponmesh_3 (Variables|Default|GetWeaponMesh))
  (bind _returnvalue (Transformation|GetWorldLocation _playercamera))
  (bind _returnvalue_2 (Transformation|GetSocketLocation _weaponmesh_2 "Muzzle"))
  (bind _returnvalue_3 (Transformation|GetSocketLocation _weaponmesh_3 "Muzzle"))
  (bind _returnvalue_4 (Pawn|GetControlRotation _owning_character :!class /Script/Engine.Pawn))
  (bind _returnvalue_5 (Transformation|GetSocketLocation _weaponmesh "Muzzle"))
  (bind (_x _y _z) (Math|Vector|BreakVector _returnvalue_2))
  (bind (_x_2 _y_2 _z_2) (Math|Vector|BreakVector _returnvalue_5))
  (bind _returnvalue_6 (Math|Vector|GetForwardVector _returnvalue_4))
  (bind _returnvalue_7 (* _returnvalue_6 1e+04))
  (bind _returnvalue_8 (+ _returnvalue _returnvalue_7))
  (bind (_outhit _returnvalue_9) (Collision|LineTraceByChannel _returnvalue _returnvalue_8 "TraceTypeQuery3" true 0 "None"))
  (if _returnvalue_9
    (return (Math|Transform|MakeTransform (Math|Vector|MakeVector _x_2 (+ _y_2 (Math|Random|RandomFloatinRange -1.0 1.0)) _z_2) (Math|Conversions|RotationFromXVector (Class|KismetMathLibrary|RandomUnitVectorinCone (Math|Vector|GetForwardVector (Math|Rotator|FindLookatRotation _returnvalue_3 (.ImpactPoint (Collision|BreakHitResult _outhit)))) 0.05))))
    (else
      (return (Math|Transform|MakeTransform (Math|Vector|MakeVector _x (+ _y (Math|Random|RandomFloatinRange -1.0 1.0)) _z) (Math|Conversions|RotationFromXVector (Class|KismetMathLibrary|RandomUnitVectorinCone (Math|Vector|GetForwardVector (Math|Rotator|FindLookatRotation _returnvalue_3 _returnvalue_8)) 0.05)))))))

(fn OnRepPlayerCamera)

(fn ServerStartFire
  (Networking|SwitchHasAuthority
    (:Authority
      (Development|PrintString "Server"))
    (:Remote
      (Development|PrintString "Client"))))

(fn OnRepOwningCharacter)

(fn CalcaulateShootingInfoServer
  (bind _playercamera (Variables|Default|GetPlayerCamera))
  (bind _owning_character (Variables|Default|GetOwning%20Character))
  (bind _weaponmesh (Variables|Default|GetWeaponMesh))
  (bind _returnvalue (Transformation|GetSocketLocation _weaponmesh "Muzzle"))
  (bind _returnvalue_2 (Transformation|GetWorldLocation _playercamera))
  (bind _returnvalue_3 (Pawn|GetControlRotation _owning_character :!class /Script/Engine.Pawn))
  (bind _returnvalue_4 (Math|Vector|GetForwardVector _returnvalue_3))
  (bind _returnvalue_5 (* _returnvalue_4 1e+04))
  (bind _returnvalue_6 (+ _returnvalue_2 _returnvalue_5))
  (bind (_outhit _returnvalue_7) (Collision|LineTraceByChannel _returnvalue_2 _returnvalue_6 "TraceTypeQuery3" true 0 "None"))
  (if _returnvalue_7
    (return (Math|Transform|MakeTransform _returnvalue (Math|Rotator|FindLookatRotation _returnvalue (.ImpactPoint (Collision|BreakHitResult _outhit)))))
    (else
      (return (Math|Transform|MakeTransform _returnvalue (Math|Rotator|FindLookatRotation _returnvalue _returnvalue_6))))))

(fn RandomizeVector
  (params (InVec :type Vector))
  (bind (_x _y _z) (Math|Vector|BreakVector InVec))
  (return (Math|Vector|MakeVector (+ _x (Math|Random|RandomFloatinRange -5.0 5.0)) (+ _y (Math|Random|RandomFloatinRange -5.0 5.0)) (+ _z (Math|Random|RandomFloatinRange -5.0 5.0)))))