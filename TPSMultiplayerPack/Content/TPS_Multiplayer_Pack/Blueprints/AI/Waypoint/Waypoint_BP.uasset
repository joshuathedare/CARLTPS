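; Waypoint actor that defines a spline path, filed under AI, with a visible marker at each point.
; The construction script loops over the spline points, placing a material billboard with query-only collision at each.
; When SnapToGround is on, SnapToGroundF line-traces vertically on Visibility and moves each point to just above the hit, keeping its X and Y.
; The actor has no active runtime logic.
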(event EventBeginPlay)

(event Collision|EventActorBeginOverlap
  (params (OtherActor :type Actor%20Object%20Reference)))

(event EventTick
  (params (DeltaSeconds :type Float%20%28single-precision%29)))

(fn ConstructionScript
  (for _index (range 0 (Spline|GetNumberOfSplinePoints (Variables|Default|GetSpline)))
    (if (Variables|Default|GetSnapToGround)
      (bind _returnvalue (CallFunction|SnaptoGroundF (Spline|GetLocationatSplinePoint (Variables|Default|GetSpline) _index "World") (Spline|GetLocationatSplinePoint (Variables|Default|GetSpline) _index "World") (.X (Math|Vector|BreakVector (Spline|GetLocationatSplinePoint (Variables|Default|GetSpline) _index "World"))) (.Y (Math|Vector|BreakVector (Spline|GetLocationatSplinePoint (Variables|Default|GetSpline) _index "World"))) _index)))
    (bind _returnvalue_2 (AddComponent|AddMaterialBillboardComponent true (Math|Transform|MakeTransform (Math|Vector|SelectVector _returnvalue (Spline|GetLocationatSplinePoint (Variables|Default|GetSpline) _index "World") (Variables|Default|GetSnapToGround)))))
    (Class|MaterialBillboardComponent|AddElement _returnvalue_2 "/Game/TPS_Multiplayer_Pack/Blueprints/AI/Waypoint/Waypoints_Mt.Waypoints_Mt" 0 false 5e+01 5e+01)
    (Collision|SetCollisionEnabled _returnvalue_2 "QueryOnly")))

(fn SnaptoGroundF
  (params (A :type Vector) (A2 :type Vector) (X :type Float%20%28single-precision%29) (Y :type Float%20%28single-precision%29) (PointIndex :type Integer))
  (bind _outhit (Collision|LineTraceByChannel (+ A "0, 0,50000.000000") (+ A2 "0, 0,-50000.000000") "TraceTypeQuery1" false 0 "None" true "(R=1.000000,G=0.000000,B=0.000000,A=1.000000)" "(R=0.000000,G=1.000000,B=0.000000,A=1.000000)" 5.0))
  (Spline|SetLocationatSplinePoint (Variables|Default|GetSpline) PointIndex (Math|Vector|MakeVector X Y (+ (.Z (Math|Vector|BreakVector (.impactpoint _outhit))) 2e+01)) "World" true)
  (return (Math|Vector|MakeVector X Y (+ (.Z (Math|Vector|BreakVector (.impactpoint _outhit))) 2e+01))))